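; Double-leaf elevator door that swings open when the first-person character enters its trigger box, if Valve01 is on.
; Leaving the box reverses the timeline and sets a closing flag, which makes the timeline's finish fire OnDoorClosed; the flag is never cleared here.
; With the valve off, entering plays a separate one-time timeline on the leaves.
; Both timelines use FlipFlop to update the mirrored yaw rotations on alternate ticks.
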(event `self.Box.OnComponentBeginOverlap`
  (params (OverlappedComponent :type "PrimitiveComponent Object Reference") (OtherActor :type "Actor Object Reference") (OtherComp :type "PrimitiveComponent Object Reference") (OtherBodyIndex :type Integer) (bFromSweep :type Boolean) (SweepResult :type "HitResult Structure (by ref)"))
  (cast `/Game/FirstPerson/Blueprints/BP_FirstPersonCharacter` OtherActor)
  (if (`self.IsValve01On`)
    (bind (_direction _newtrack_0) (`Timeline|Timeline` :!label _label)
      (:`Update`
        (`/Engine/EditorBlueprintResources/StandardMacros.FlipFlop`
          (:`A`
            (`SceneComponent.K2_SetRelativeRotation` (`self.Boolean_6B79A90A`) (`KismetMathLibrary.MakeRotator` 0.0 0.0 (* _newtrack_0 -1.0)) false false))
          (:`B`
            (`SceneComponent.K2_SetRelativeRotation` (`self.Boolean_D191D969`) (`KismetMathLibrary.MakeRotator` 0.0 0.0 _newtrack_0) false false))))
      (:`Finished`
        (if (stale `self.Box.OnComponentEndOverlap` _output_get)
          (`self.OnDoorClosed`))))
    (else
      (`/Engine/EditorBlueprintResources/StandardMacros.DoOnce` false
        (:`Completed`
          (bind (_direction_2 _newtrack_0_2) (`Timeline|Timeline_0`)
            (:`Update`
              (`/Engine/EditorBlueprintResources/StandardMacros.FlipFlop`
                (:`A`
                  (`SceneComponent.K2_SetRelativeRotation` (`self.Boolean_6B79A90A`) (`KismetMathLibrary.MakeRotator` 0.0 0.0 (* _newtrack_0_2 -1.0)) false false))
                (:`B`
                  (`SceneComponent.K2_SetRelativeRotation` (`self.Boolean_D191D969`) (`KismetMathLibrary.MakeRotator` 0.0 0.0 _newtrack_0_2) false false))))))))))

(event `self.Box.OnComponentEndOverlap`
  (params (OverlappedComponent :type "PrimitiveComponent Object Reference") (OtherActor :type "Actor Object Reference") (OtherComp :type "PrimitiveComponent Object Reference") (OtherBodyIndex :type Integer))
  (cast `/Game/FirstPerson/Blueprints/BP_FirstPersonCharacter` OtherActor)
  (if (`self.IsValve01On`)
    (bind _output_get (set `self.IsDoorClosing` true))
    (goto _label :!via `Reverse`)))

(fn `UserConstructionScript`)