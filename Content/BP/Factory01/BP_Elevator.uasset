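; BP_Elevator is an elevator that moves once its door closes with the player inside.
; A box collision tracks whether the first-person character is inside.
; On BeginPlay it binds to the ElevatorDoor's OnDoorClosed event, which checks that flag and plays a timeline.
; The timeline drives the relative Z location of a cylinder component; it only plays forward, with no return trip in this graph.
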(event `self.BoxCollision.OnComponentBeginOverlap`
  (params (OverlappedComponent :type "PrimitiveComponent Object Reference") (OtherActor :type "Actor Object Reference") (OtherComp :type "PrimitiveComponent Object Reference") (OtherBodyIndex :type Integer) (bFromSweep :type Boolean) (SweepResult :type "HitResult Structure (by ref)"))
  ; Enter/Exit Collision with player check
  (cast `/Game/FirstPerson/Blueprints/BP_FirstPersonCharacter` OtherActor)
  (set `self.IsPlayerInside` true))

(event `self.BoxCollision.OnComponentEndOverlap`
  (params (OverlappedComponent :type "PrimitiveComponent Object Reference") (OtherActor :type "Actor Object Reference") (OtherComp :type "PrimitiveComponent Object Reference") (OtherBodyIndex :type Integer))
  ; Enter/Exit Collision with player check
  (cast `/Game/FirstPerson/Blueprints/BP_FirstPersonCharacter` OtherActor)
  (set `self.IsPlayerInside` false))

(event `OnDoorClosed_Event`
  ; OnDoorClosed Event
  (if (`self.IsPlayerInside`)
    (bind (_direction _newtrack_0) (`Timeline|Timeline`)
      (:`Update`
        (`SceneComponent.K2_SetRelativeLocation` (`self.Cylinder_00FFBB1D`) (`KismetMathLibrary.MakeVector` 0.0 0.0 _newtrack_0) false false)))))

(event `self.ReceiveBeginPlay`
  ; OnDoorClosed Event
  (add `/Game/BP/Factory01/BP_ElevatorDoor.OnDoorClosed` (`self.ElevatorDoor`) (delegate `OnDoorClosed_Event`)))

(fn `UserConstructionScript`)