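; BP_Valve is an interactable valve that the player turns by holding interact to switch on one condition for an elevator.
; A box overlap registers the valve as the player controller's LastInteractObject and enables interaction while the player is inside.
; BeginInteract plays a timeline that rotates the valve's yaw; releasing or leaving pauses it, so progress is kept.
; When the timeline finishes, it sets IsValve01On on the ElevatorOn reference.
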(event `self.Box.OnComponentBeginOverlap`
  (params (OverlappedComponent :type "PrimitiveComponent Object Reference") (OtherActor :type "Actor Object Reference") (OtherComp :type "PrimitiveComponent Object Reference") (OtherBodyIndex :type Integer) (bFromSweep :type Boolean) (SweepResult :type "HitResult Structure (by ref)"))
  ; Enter/Exit Collision
  (bind _asbp_first_person_character (cast `/Game/FirstPerson/Blueprints/BP_FirstPersonCharacter` OtherActor))
  (bind _asbp_first_person_player_controller (cast `/Game/FirstPerson/Blueprints/BP_FirstPersonPlayerController` (`Pawn.GetController` _asbp_first_person_character)))
  (set `/Game/FirstPerson/Blueprints/BP_FirstPersonPlayerController.LastInteractObject` self _asbp_first_person_player_controller)
  (set `self.IsInteractable` true))

(event `self.Box.OnComponentEndOverlap`
  (params (OverlappedComponent :type "PrimitiveComponent Object Reference") (OtherActor :type "Actor Object Reference") (OtherComp :type "PrimitiveComponent Object Reference") (OtherBodyIndex :type Integer))
  ; Enter/Exit Collision
  (cast `/Game/FirstPerson/Blueprints/BP_FirstPersonCharacter` OtherActor)
  (set `self.IsInteractable` false)
  (bind (_direction _newtrack_0) (`Timeline|Timeline` :!via `Stop` :!label _label)
    (:`Update`
      (`SceneComponent.K2_SetRelativeRotation` (`self.Valve`) (`KismetMathLibrary.MakeRotator` 0.0 0.0 _newtrack_0) false false))
    (:`Finished`
      (set `/Game/BP/Factory01/BP_ElevatorDoor.IsValve01On` true (`self.ElevatorOn`)))))

(event `/Game/BP/Interact_Interface.BeginInteract`
  (if (`self.IsInteractable`)
    (goto _label)))

(event `/Game/BP/Interact_Interface.EndInteract`
  (goto _label :!via `Stop`))

(fn `UserConstructionScript`)