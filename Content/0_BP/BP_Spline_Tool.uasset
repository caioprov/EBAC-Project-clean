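; BP_Spline_Tool is a construction-script tool that lays spline mesh components along a spline at a fixed spacing, apparently for pipes.
; Each component takes its transform from the spline, with slight random variation in Y and Z scale, and joins the SplineMeshes array.
; A tangent dot-product angle test classifies each segment: straighter ones get the first mesh from Meshes, while sharper bends only record curve index and type, without assigning a mesh.
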(fn `UserConstructionScript`
  (bind _returnvalue (`KismetMathLibrary.RandomFloatInRange` 0.95 1.05))
  (bind _spline (`self.Spline`))
  (bind _distance (`self.Distance`))
  (bind (_relative_transform_scale_x _relative_transform_scale_y _relative_transform_scale_z) (`KismetMathLibrary.BreakVector` (`self.Relative Transform Scale`)))
  (bind _returnvalue_2 (/ _distance 4.0))
  ; Amount of spline meshes
  (for _index (range (+ (`KismetMathLibrary.FTrunc` (/ (`SplineComponent.GetSplineLength` _spline) _distance)) 1))
    (set `self.Index` _index)
    (bind _returnvalue_3 (* _index _distance))
    (bind (_returnvalue_location _returnvalue_rotation) (`KismetMathLibrary.BreakTransform` (`SplineComponent.GetTransformAtDistanceAlongSpline` _spline _returnvalue_3 "Local" false)))
    (bind _returnvalue_4 (`AddComponent|NODE_AddSplineMeshComponent-0` :`RelativeTransform` (`KismetMathLibrary.MakeTransform` _returnvalue_location _returnvalue_rotation (`KismetMathLibrary.MakeVector` _relative_transform_scale_x (* _relative_transform_scale_y _returnvalue) (* _relative_transform_scale_z _returnvalue)))))
    (`KismetArrayLibrary.Array_Add` (`self.SplineMeshes`) _returnvalue_4)
    (bind _returnvalue_5 (+ _returnvalue_3 (/ _distance 2.0)))
    (if (< (`KismetMathLibrary.RadiansToDegrees` (`KismetMathLibrary.Acos` (`KismetMathLibrary.FClamp` (`KismetMathLibrary.Dot_VectorVector` (`KismetMathLibrary.Normal` (`SplineComponent.GetTangentAtDistanceAlongSpline` _spline (- _returnvalue_5 _returnvalue_2) "Local")) (`KismetMathLibrary.Normal` (`SplineComponent.GetTangentAtDistanceAlongSpline` _spline (+ _returnvalue_5 _returnvalue_2) "Local")))))) 15.0)
      (set `self.TypeofPipe` 0)
      (`StaticMeshComponent.SetStaticMesh` _returnvalue_4 (`|ConvertAsset` (`|GetArrayItem` (`self.Meshes`) (`self.TypeofPipe`))))
      (else
        (set `self.IndexCurves` (`self.Index`))
        (set `self.TypeofPipe` 1)))))