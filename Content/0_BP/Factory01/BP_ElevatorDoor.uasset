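; Elevator double door that swings open when the first-person player enters its trigger box, provided Valve01 has been turned.
; A timeline yaws the two panels in opposite directions, with a FlipFlop updating one panel per tick.
; Leaving the box reverses the timeline and calls OnDoorClosed when it finishes.
; Without the valve turned, a second timeline plays a one-time failed-opening animation.
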(event `self.Box.OnComponentBeginOverlap`
  (params (OverlappedComponent :type "PrimitiveComponent Object Reference") (OtherActor :type "Actor Object Reference") (OtherComp :type "PrimitiveComponent Object Reference") (OtherBodyIndex :type Integer) (bFromSweep :type Boolean) (SweepResult :type "HitResult Structure (by ref)"))
  ; Enter/Exit Collision
  (cast `/Game/FirstPerson/Blueprints/BP_FirstPersonCharacter` OtherActor)
  ; IsValve01Turned?
  (if (`self.IsValve01Turned`)
    ; DoorAnimation
    (bind (_direction _newtrack_0) (`Timeline|Timeline` :!label _label)
      (:`Update`
        (`/Engine/EditorBlueprintResources/StandardMacros.FlipFlop`
          (:`A`
            (`SceneComponent.K2_SetRelativeRotation` (`self.Boolean_6B79A90A`) (`KismetMathLibrary.MakeRotator` 0.0 0.0 (* _newtrack_0 -1.0)) false false))
          (:`B`
            (`SceneComponent.K2_SetRelativeRotation` (`self.Boolean_D191D969`) (`KismetMathLibrary.MakeRotator` 0.0 0.0 _newtrack_0) false false))))
      (:`Finished`
        ; IsDoorClosing?                                                                                                                              CallOnDoorClosed Event!
        (if (stale `self.Box.OnComponentEndOverlap` _output_get)
          (`self.OnDoorClosed`))))
    (else
      ; Door Failling to open due to no resources
      (`/Engine/EditorBlueprintResources/StandardMacros.DoOnce` false
        (:`Completed`
          (bind (_direction_2 _newtrack_0_2) (`Timeline|Timeline_0`)
            (:`Update`
              (`/Engine/EditorBlueprintResources/StandardMacros.FlipFlop`
                (:`A`
                  (`SceneComponent.K2_SetRelativeRotation` (`self.Boolean_6B79A90A`) (`KismetMathLibrary.MakeRotator` 0.0 0.0 (* _newtrack_0_2 -1.0)) false false))
                (:`B`
                  (`SceneComponent.K2_SetRelativeRotation` (`self.Boolean_D191D969`) (`KismetMathLibrary.MakeRotator` 0.0 0.0 _newtrack_0_2) false false))))))))))

(event `self.Box.OnComponentEndOverlap`
  (params (OverlappedComponent :type "PrimitiveComponent Object Reference") (OtherActor :type "Actor Object Reference") (OtherComp :type "PrimitiveComponent Object Reference") (OtherBodyIndex :type Integer))
  ; Enter/Exit Collision
  (cast `/Game/FirstPerson/Blueprints/BP_FirstPersonCharacter` OtherActor)
  ; IsValve01Turned?
  (if (`self.IsValve01Turned`)
    ; IsDoorClosing?                                                                                                                              CallOnDoorClosed Event!
    (bind _output_get (set `self.IsDoorClosing` true))
    (goto _label :!via `Reverse`)))

(fn `UserConstructionScript`)