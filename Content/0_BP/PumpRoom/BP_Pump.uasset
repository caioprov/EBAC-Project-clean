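; Pump Blueprint in the pump room that animates a cylinder's height as a lava tank animation, responding to Valve02.
; On BeginPlay it binds the valve's turn event and starts a Timeline, whose completion drives a FlipFlop alternating play and reverse for a back-and-forth cycle.
; Once the valve is turned, a check on the FlipFlop state hands the cylinder to a second Timeline that restarts itself whenever it finishes.
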(event `OnValveTurned`
  ; OnValveTurned Event
  (set `self.IsValve02Turned` true))

(event `self.ReceiveBeginPlay`
  ; OnValveTurned Event
  (add `/Game/0_BP/BP_Valve.OnValveTurned` (`self.Valve02`) (delegate `OnValveTurned`))
  ; LavaTankAnimation
  (bind (_direction _newtrack_0) (`Timeline|Timeline` :!via `PlayFromStart` :!label _label)
    (:`Update`
      (`SceneComponent.K2_SetRelativeLocation` (`self.Cylinder_D03C4943`) (`KismetMathLibrary.MakeVector` 0.0 0.0 _newtrack_0) false false))
    (:`Finished`
      (if (`self.IsValve02Turned`)
        (if (stale _isa)
          (bind (_direction_2 _newtrack_0_2) (`Timeline|Timeline_0` :!via `PlayFromStart` :!label _label_2)
            (:`Update`
              (`SceneComponent.K2_SetRelativeLocation` (`self.Cylinder_D03C4943`) (`KismetMathLibrary.MakeVector` 0.0 0.0 _newtrack_0_2) false false))
            (:`Finished`
              (goto _label_2 :!via `PlayFromStart`)))
          (else
            (bind _isa (`/Engine/EditorBlueprintResources/StandardMacros.FlipFlop` :!label _label_3)
              (:`A`
                (goto _label))
              (:`B`
                (goto _label :!via `Reverse`)))))
        (else
          (goto _label_3))))))

(fn `UserConstructionScript`)