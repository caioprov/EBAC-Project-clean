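; BP_Button is an interactable button that the first-person player can press while standing inside its trigger box.
; Entering the box registers the button as the player controller's LastInteractObject and sets IsInteractable, while leaving clears only that flag.
; BeginInteract checks the flag and, if set, fires the OnButtonPressed dispatcher, leaving the response to whatever is bound to it.
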(event `self.Box.OnComponentBeginOverlap`
  (params (OverlappedComponent :type "PrimitiveComponent Object Reference") (OtherActor :type "Actor Object Reference") (OtherComp :type "PrimitiveComponent Object Reference") (OtherBodyIndex :type Integer) (bFromSweep :type Boolean) (SweepResult :type "HitResult Structure (by ref)"))
  ; Enter/Exit Collision
  (bind _asbp_first_person_character (cast `/Game/FirstPerson/Blueprints/BP_FirstPersonCharacter` OtherActor))
  (bind _asbp_first_person_player_controller (cast `/Game/FirstPerson/Blueprints/BP_FirstPersonPlayerController` (`Pawn.GetController` _asbp_first_person_character)))
  (set `/Game/FirstPerson/Blueprints/BP_FirstPersonPlayerController.LastInteractObject` self _asbp_first_person_player_controller)
  (set `self.IsInteractable` true))

(event `self.Box.OnComponentEndOverlap`
  (params (OverlappedComponent :type "PrimitiveComponent Object Reference") (OtherActor :type "Actor Object Reference") (OtherComp :type "PrimitiveComponent Object Reference") (OtherBodyIndex :type Integer))
  ; Enter/Exit Collision
  (cast `/Game/FirstPerson/Blueprints/BP_FirstPersonCharacter` OtherActor)
  (set `self.IsInteractable` false))

(event `/Game/0_BP/Interact_Interface.BeginInteract`
  ; IsInteractable?
  (if (`self.IsInteractable`)
    ; CallOnButtonTurnedEvent
    (`self.OnButtonPressed`)))

(fn `UserConstructionScript`)