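; BP_Spline_Tool1 is a spline tool that lays a chosen mesh along a spline in repeated segments.
; The construction script divides the spline length by Distance and adds a Spline Mesh Component for each step, including index zero and the truncated count.
; Each segment takes its start and end positions and unscaled tangents from the spline in local space, so the mesh bends along the curve.
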(fn `UserConstructionScript`
  (bind _spline (`self.Spline`))
  (bind _distance (`self.Distance`))
  (for _index (range (+ (`KismetMathLibrary.FTrunc` (/ (`SplineComponent.GetSplineLength` _spline) _distance)) 1))
    (bind _returnvalue (`AddComponent|NODE_AddSplineMeshComponent-0`))
    (`StaticMeshComponent.SetStaticMesh` _returnvalue (`self.Meshes`))
    (bind _returnvalue_2 (* _index _distance))
    (bind _returnvalue_3 (* (+ _index 1) _distance))
    (`SplineMeshComponent.SetStartAndEnd` _returnvalue (`SplineComponent.GetLocationAtDistanceAlongSpline` _spline _returnvalue_2 "Local") (`SplineComponent.GetTangentAtDistanceAlongSpline` _spline _returnvalue_2 "Local") (`SplineComponent.GetLocationAtDistanceAlongSpline` _spline _returnvalue_3 "Local") (`SplineComponent.GetTangentAtDistanceAlongSpline` _spline _returnvalue_3 "Local") true)))